(event OnComponentBeginOverlap(BoxLeft)
  (params (OverlappedComponent :type Primitive%20Component%20Object%20Reference) (OtherActor :type Actor%20Object%20Reference) (OtherComp :type Primitive%20Component%20Object%20Reference) (OtherBodyIndex :type Integer) (bFromSweep :type Boolean) (SweepResult :type Hit%20Result%20Structure%20%28by%20ref%29))
  ;[1 1 1] Begin/End Overlap
  (if (== OtherActor (Game|Player|GetPlayerPawn 0))
    (Variables|Default|SetIsCanInteract true)))

(event OnComponentBeginOverlap(BoxRight)
  (params (OverlappedComponent :type Primitive%20Component%20Object%20Reference) (OtherActor :type Actor%20Object%20Reference) (OtherComp :type Primitive%20Component%20Object%20Reference) (OtherBodyIndex :type Integer) (bFromSweep :type Boolean) (SweepResult :type Hit%20Result%20Structure%20%28by%20ref%29))
  ;[1 1 1] Begin/End Overlap
  (if (== OtherActor (Game|Player|GetPlayerPawn 0))
    (Variables|Default|SetIsCanInteract true)))

(event OnComponentEndOverlap(BoxLeft)
  (params (OverlappedComponent :type Primitive%20Component%20Object%20Reference) (OtherActor :type Actor%20Object%20Reference) (OtherComp :type Primitive%20Component%20Object%20Reference) (OtherBodyIndex :type Integer))
  ;[1 1 1] Begin/End Overlap
  (if (== OtherActor "/Game/Blueprints/MainCharacter/MainCharacter.MainCharacter")
    (Variables|Default|SetIsCanInteract false)))

(event OnComponentEndOverlap(BoxRight)
  (params (OverlappedComponent :type Primitive%20Component%20Object%20Reference) (OtherActor :type Actor%20Object%20Reference) (OtherComp :type Primitive%20Component%20Object%20Reference) (OtherBodyIndex :type Integer))
  ;[1 1 1] Begin/End Overlap
  (if (== OtherActor "/Game/Blueprints/MainCharacter/MainCharacter.MainCharacter")
    (Variables|Default|SetIsCanInteract false)))

(event EventInteractInterfaceFunc
  ;[1 1 1] EventInteract
  (if (Variables|Default|GetIsCanInteract)
    (if (Variables|Default|GetIsDoorOpen)
      (Variables|Default|SetIsDoorOpen false)
      (bind (_direction _openfront _openback) (Timeline|Timeline_0 Reverse)
        (:Update
          (Transformation|SetRelativeRotation (Variables|Default|GetScene) (Math|Rotator|MakeRotator 0.0 0.0 (Math|Float|SelectFloat _openfront _openback (Math|Float|InRange(Float) (Variables|Default|GetAngleOnOpen) -9e+01 9e+01))) false false)
          (Utilities|FlowControl|DoOnce false :!label _label
            (:Completed
              (Collision|SetCollisionEnabled (Variables|Default|GetCube) "NoCollision"))))
        (:Finished
          (Collision|SetCollisionEnabled (Variables|Default|GetCube) "QueryAndPhysics")
          (goto _label Reset)))
      (else
        (Variables|Default|SetIsDoorOpen true)
        (Variables|Default|SetAngleOnOpen (.Yaw (Math|Rotator|BreakRotator (.rotation (Transformation|GetActorTransform (Game|Player|GetPlayerPawn 0))))))
        (Timeline|Timeline_0 Play)))))

(event EventTick
  (params (DeltaSeconds :type Float%20%28single-precision%29)))

(event EventBeginPlay
  (Variables|Default|SetOutputColor (Utilities|Struct|MakeLinearColor (Math|Random|RandomFloat) (Math|Random|RandomFloat) (Math|Random|RandomFloat) 1.0)))

(fn ConstructionScript)