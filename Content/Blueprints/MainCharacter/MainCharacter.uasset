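; MainCharacter is the player character Blueprint, handling movement, camera look and a toggleable flashlight from mapped input.
; Axis inputs drive movement along the actor's forward and right vectors and controller pitch and yaw.
; Action inputs trigger jumping, hold-to-crouch, and hold-to-run, which adds and then subtracts an acceleration value from max walk speed.
; The flashlight input flips visibility and a state flag while playing on or off sounds at the light's location.
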(event Input|ActionEvents|InputActionJump
  (params (Key :type Key%20Structure :default "None"))
  ;[1 1 1] MovementActions
  (:Pressed
    (Character|Jump)))

(event Input|ActionEvents|InputActionCrounch
  (params (Key :type Key%20Structure :default "None"))
  ;[1 1 1] MovementActions
  (:Pressed
    (Character|Crouch))
  (:Released
    (Character|UnCrouch)))

(event Input|ActionEvents|InputActionFlashLight
  (params (Key :type Key%20Structure :default "None"))
  ;[1 1 1] Flashlight
  (:Pressed
    (if (Variables|Default|GetIsFlashlightON)
      (Audio|PlaySoundatLocation "/Game/Sounds/Flashlight/FlashLight_OFF.FlashLight_OFF" (Transformation|GetWorldLocation (Variables|Default|GetFlashLight)) "0, 0, 0" 1.0 1.0 0.0 0 0 0)
      (Rendering|SetVisibility (Variables|Default|GetFlashLight) false false)
      (Variables|Default|SetIsFlashlightON false)
      (else
        (Audio|PlaySoundatLocation "/Game/Sounds/Flashlight/FlashLight_ON.FlashLight_ON" (Transformation|GetWorldLocation (Variables|Default|GetFlashLight)) "0, 0, 0" 1.0 1.0 0.0 0 0 0)
        (Rendering|SetVisibility (Variables|Default|GetFlashLight) true false)
        (Variables|Default|SetIsFlashlightON true)))))

(event Input|ActionEvents|InputActionRun
  (params (Key :type Key%20Structure :default "None"))
  (bind _charactermovement (Variables|Character|GetCharacterMovement))
  (bind _charactermovement_2 (Variables|Character|GetCharacterMovement))
  (bind _accelerations (Variables|Default|GetAccelerations))
  ;[1 1 1] MovementActions
  (:Pressed
    (Variables|/Script/Engine.CharacterMovementComponent|SetMaxWalkSpeed _charactermovement (+ _accelerations (Class|MovementComponent|GetMaxSpeed _charactermovement_2))))
  (:Released
    (Variables|/Script/Engine.CharacterMovementComponent|SetMaxWalkSpeed _charactermovement (- (Class|MovementComponent|GetMaxSpeed _charactermovement_2) _accelerations))))

(event Input|AxisEvents|InputAxisMoveForwardandBack
  (params (AxisValue :type Float%20%28single-precision%29))
  ;[1 1 1] Movement
  (Pawn|Input|AddMovementInput (Transformation|GetActorForwardVector) AxisValue false))

(event Input|AxisEvents|InputAxisMoveRightandLeft
  (params (AxisValue :type Float%20%28single-precision%29))
  ;[1 1 1] Movement
  (Pawn|Input|AddMovementInput (Transformation|GetActorRightVector) AxisValue false))

(event Input|AxisEvents|InputAxisLookUpandDown
  (params (AxisValue :type Float%20%28single-precision%29))
  ;[1 1 1] Camera
  (Pawn|Input|AddControllerPitchInput AxisValue))

(event Input|AxisEvents|InputAxisLookHorizontal
  (params (AxisValue :type Float%20%28single-precision%29))
  ;[1 1 1] Camera
  (Pawn|Input|AddControllerYawInput AxisValue))

(fn ConstructionScript)