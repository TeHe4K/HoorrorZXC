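; AI controller for a test enemy, judging by its name, that patrols between the TargetPoint actors in the level.
; Each Tick it gathers all TargetPoints and issues an AI MoveTo toward the one at PointIndex.
; A successful move advances the index and wraps it to zero after the last point, through a DoN node that caps advances at 100.
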(event EventBeginPlay)

(event EventTick
  (params (DeltaSeconds :type Float%20%28single-precision%29))
  (bind _outactors (Actor|GetAllActorsOfClass "/Script/Engine.TargetPoint"))
  (AI|AIMoveTo 0 "0, 0, 0" (Utilities|Array|Get(acopy) _outactors (Variables|Default|GetPointIndex)) 5.0 false
    (:OnSuccess
      (Utilities|FlowControl|DoN 100
        (:Exit
          (Math|Integer|IncrementInt (Variables|Default|GetPointIndex)
            (:%20%20
              (if (== (Utilities|Array|Length _outactors) (Variables|Default|GetPointIndex))
                (Variables|Default|SetPointIndex 0)))))))))

(fn ConstructionScript)