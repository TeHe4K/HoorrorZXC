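; AI controller for a test enemy that keeps its pawn moving and steers it when something blocks the way.
; Each Tick, a visibility line trace runs a short distance along the pawn's forward vector.
; A hit rotates the stored Direction vector by a small fixed step per frame, so turn speed depends on frame rate.
; Direction feeds movement input every Tick, with no navigation or target logic.
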(event EventBeginPlay)

(event EventTick
  (params (DeltaSeconds :type Float%20%28single-precision%29))
  (bind _returnvalue (Pawn|GetControlledPawn))
  (bind _returnvalue_2 (Transformation|GetActorLocation _returnvalue))
  (bind _returnvalue_3 (Collision|LineTraceByChannel _returnvalue_2 (+ _returnvalue_2 (* (Transformation|GetActorForwardVector _returnvalue) 5e+02)) "TraceTypeQuery1" false 0 "None"))
  (if _returnvalue_3
    (Variables|Default|SetDirection (Math|Vector|RotateVector (Variables|Default|GetDirection) "0,3.000000,0.000000")))
  (Pawn|Input|AddMovementInput _returnvalue (Variables|Default|GetDirection) 1.0 false))

(fn ConstructionScript)