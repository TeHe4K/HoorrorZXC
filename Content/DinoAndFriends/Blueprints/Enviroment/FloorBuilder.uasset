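; FloorBuilder is an environment Blueprint that generates a tiled grid of mesh instances, named as a floor builder.
; Its construction script runs nested loops over NumX and NumY, adding instances to a Hierarchical Instanced Static Mesh at fixed, even spacing.
; The second axis maps to Z rather than Y, so the grid lies in the actor's local XZ plane.
; The event graph holds only disabled placeholder events, with no runtime logic.
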(event EventBeginPlay)

(event Collision|EventActorBeginOverlap
  (params (OtherActor :type Actor%20Object%20Reference)))

(event EventTick
  (params (DeltaSeconds :type Float%20%28single-precision%29)))

(fn ConstructionScript
  (for _index (range 0 (- (Variables|Default|GetNumX) 1))
    (Variables|Default|SetLoopX _index)
    (for _index_2 (range 0 (- (Variables|Default|GetNumY) 1))
      (Variables|Default|SetLoopY _index_2)
      (Components|InstancedStaticMesh|AddInstance (Variables|Default|GetHierarchicalInstancedStaticMesh) (Math|Transform|MakeTransform (Math|Vector|MakeVector (* (Variables|Default|GetLoopX) 4e+02) 0.0 (* (Variables|Default|GetLoopY) 4e+02)) "0, 0, 0" "1,1,1")))))