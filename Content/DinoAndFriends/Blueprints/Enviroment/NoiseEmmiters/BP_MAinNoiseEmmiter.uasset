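; Noise emitter actor that plays a data-driven sound in the world and signals the player when it can be interacted with.
; Construction script looks up its row in DT_NoiseEmmiters to set the mesh, material, sound and attenuation.
; TriggerBox overlaps send can/cannot interact messages to the player pawn.
; SetSoundToNone clears the audio component's sound, while SetSoundToDefault is an empty stub.
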(event OnComponentBeginOverlap(TriggerBox)
  (params (OverlappedComponent :type Primitive%20Component%20Object%20Reference) (OtherActor :type Actor%20Object%20Reference) (OtherComp :type Primitive%20Component%20Object%20Reference) (OtherBodyIndex :type Integer) (bFromSweep :type Boolean) (SweepResult :type Hit%20Result%20Structure%20%28by%20ref%29))
  (bind _returnvalue (Game|Player|GetPlayerPawn 0))
  (if (== OtherActor _returnvalue)
    (Class|BPIInteracte|CanInteract(Message) _returnvalue)))

(event OnComponentEndOverlap(TriggerBox)
  (params (OverlappedComponent :type Primitive%20Component%20Object%20Reference) (OtherActor :type Actor%20Object%20Reference) (OtherComp :type Primitive%20Component%20Object%20Reference) (OtherBodyIndex :type Integer))
  (bind _returnvalue (Game|Player|GetPlayerPawn 0))
  (if (== OtherActor _returnvalue)
    (Class|BPIInteracte|CanNotInteract(Message) _returnvalue)))

(event EventBeginPlay)

(event Collision|EventActorBeginOverlap
  (params (OtherActor :type Actor%20Object%20Reference)))

(event EventTick
  (params (DeltaSeconds :type Float%20%28single-precision%29)))

(fn ConstructionScript
  (bind _staticmesh (Variables|Default|GetStaticMesh))
  (bind _noise (Variables|Default|GetNoise))
  (bind _returnvalue (Utilities|GetDataTableRow "/Game/DinoAndFriends/Blueprints/Enviroment/NoiseEmmiters/DT_NoiseEmmiters.DT_NoiseEmmiters" (Variables|Default|GetNoiseEmmiterRowName))
    (:then
      (Components|StaticMesh|SetStaticMesh _staticmesh (.SM_EmmiterModel (Utilities|Struct|BreakStruct_NoiseEmmiter _returnvalue)))
      (Rendering|Material|SetMaterial _staticmesh 0 (.Mat_EmmiterMaterial (Utilities|Struct|BreakStruct_NoiseEmmiter _returnvalue)))
      (Variables|Default|SetSC%20Emmiter%20Sound (.SC_EmmiterSound (Utilities|Struct|BreakStruct_NoiseEmmiter _returnvalue)))
      (Audio|Components|Audio|SetSound _noise (.SC_EmmiterSound (Utilities|Struct|BreakStruct_NoiseEmmiter _returnvalue)))
      (Audio|Components|Audio|AdjustAttenuation _noise (Variables|/Script/Engine.SoundAttenuation|GetAttenuation (.SA_EmmiterSoundAttenuation (Utilities|Struct|BreakStruct_NoiseEmmiter _returnvalue)))))))

(fn SetSoundtoNone
  (Audio|Components|Audio|SetSound (Variables|Default|GetNoise) 0))

(fn SetSoundtoDefault)