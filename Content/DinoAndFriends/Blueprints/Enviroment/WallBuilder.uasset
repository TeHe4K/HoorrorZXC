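; WallBuilder is an environment actor that builds a straight row of wall segments, with door frames and windows at chosen indices.
; Its construction script assigns meshes to three instanced mesh components, then adds one instance per segment along local Y.
; Counters walk the door and window index arrays, so these need ascending order; door frames take priority.
; Each frame also spawns a BP_Door, using the offset as an unconverted world transform.
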(event EventBeginPlay)

(event Collision|EventActorBeginOverlap
  (params (OtherActor :type Actor%20Object%20Reference)))

(event EventTick
  (params (DeltaSeconds :type Float%20%28single-precision%29)))

(fn ConstructionScript
  (Utilities|SetMeshes
    (:Output
      (for _index (range 1 (Variables|Default|GetWallCount))
        (if (== (Utilities|Array|Get(acopy) (Variables|Default|GetWhereDoorFrames) (Variables|Default|GetDoorFrameCounter)) _index)
          (Math|Integer|IncrementInt (Variables|Default|GetDoorFrameCounter)
            (:%20%20
              (Components|InstancedStaticMesh|AddInstance (Variables|Default|GetHISM_DoorFrame) (Math|Transform|MakeTransform (Math|Vector|MakeVector 0.0 (* (- _index 1) (Variables|Default|GetWallLenght)) 0.0) "0,-270.000000, 0" "1,1,1"))
              (Utilities|SpawnDoor (Math|Transform|MakeTransform (Math|Vector|MakeVector 0.0 (+ (* (- _index 1) (Variables|Default|GetWallLenght)) (Variables|Default|GetDoorOffset)) 0.0) "0,90.000000, 0" "1,1,1"))))
          (elif (== _index (Utilities|Array|Get(acopy) (Variables|Default|GetWhereWindow) (Variables|Default|GetWindowCounter)))
            (Math|Integer|IncrementInt (Variables|Default|GetWindowCounter)
              (:%20%20
                (Components|InstancedStaticMesh|AddInstance (Variables|Default|GetHISM_Window) (Math|Transform|MakeTransform (Math|Vector|MakeVector 0.0 (* (- _index 1) (Variables|Default|GetWallLenght)) 0.0) "0,-270.000000, 0" "1,1,1"))))
            (else
              (Components|InstancedStaticMesh|AddInstance (Variables|Default|GetHISM_Wall) (Math|Transform|MakeTransform (Math|Vector|MakeVector 0.0 (* (- _index 1) (Variables|Default|GetWallLenght)) 0.0) "0,-270.000000,0.000000" "1,1,1")))))))))