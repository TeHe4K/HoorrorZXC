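; BP_CheckDoorOpenWay is a test actor that probes doors with a rotating trace and shows which way they open.
; A DoOnce on Tick replays a yaw timeline in a loop, tracing from FrontArrow to Scene1 on each update.
; Hits tagged Interactable that cast to BP_DoorForCheckNOTPLAYABLE supply IsDoorOpenFront, then receive an interact message.
; That flag picks the debug trace's hit color.
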(event EventTick
  (params (DeltaSeconds :type Float%20%28single-precision%29))
  (Utilities|FlowControl|DoOnce false :!label _label
    (:Completed
      (bind _newtrack_0 (Timeline|Timeline_0 PlayFromStart)
        (:Update
          (Transformation|SetActorRotation (Math|Rotator|MakeRotator 0.0 0.0 _newtrack_0))
          (bind (_outhit _returnvalue) (Collision|LineTraceForObjects (Transformation|GetWorldLocation (Variables|Default|GetFrontArrow)) (Transformation|GetWorldLocation (Variables|Default|GetScene1)) (Utilities|Array|MakeArray "ObjectTypeQuery1") false 0 "ForDuration" true "(R=1.000000,G=0.000000,B=0.000000,A=1.000000)" (Math|Color|SelectColor "(R=0.000000,G=1.000000,B=0.096483,A=1.000000)" "(R=1.000000,G=0.410085,B=0.000000,A=1.000000)" (Variables|Default|GetIs%20Door%20Open%20Front)) 1.0))
          (if _returnvalue
            (if (Actor|ActorHasTag (.HitActor (Collision|BreakHitResult _outhit)) "Interactable")
              (bind _asbp_door_for_check_notplayable (Utilities|Casting|CastToBP_DoorForCheckNOTPLAYABLE (.HitActor (Collision|BreakHitResult _outhit))))
              (Variables|Default|SetIs%20Door%20Open%20Front (Variables|/Game/DinoAndFriends/Blueprints/Ineractable/Door/BP_DoorForCheckNOTPLAYABLE.BP_DoorForCheckNOTPLAYABLE_C|GetIsDoorOpenFront _asbp_door_for_check_notplayable))
              (Class|IFInteracte|InteractInterfaceFunc(Message) (.HitActor (Collision|BreakHitResult _outhit))))))
        (:Finished
          (goto _label Reset))))))

(event EventBeginPlay)

(fn ConstructionScript)