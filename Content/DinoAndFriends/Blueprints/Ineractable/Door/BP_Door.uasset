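; Interactive door that the player taps to open or close, or holds to crack open and eavesdrop on the room beyond.
; Timelines swing it by the player's facing, and for listening also lock movement and glide the camera to the door.
; Linked room trigger boxes and box traces feed tag-based occupant flags.
; These pick enemy or environment audio while listening, and a horror cue plays when the player nears an occupied room.
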(event OnComponentBeginOverlap(DoorBoxFront)
  (params (OverlappedComponent :type Primitive%20Component%20Object%20Reference) (OtherActor :type Actor%20Object%20Reference) (OtherComp :type Primitive%20Component%20Object%20Reference) (OtherBodyIndex :type Integer) (bFromSweep :type Boolean) (SweepResult :type Hit%20Result%20Structure%20%28by%20ref%29))
  ;[1 1 1] Begin/End Overlap
  ;;[1 1 1] CheckPlayerCollisionBox
  (if (== OtherActor (Game|Player|GetPlayerPawn 0))
    (Variables|Default|SetIsPlayerInCheckBoxFront true)
    (CallFunction|CheckSetandActivateSoundifinRoomMore0EntitiesforManyRoom (Variables|Default|GetBackBoxesCollisionForCheckEnemy))))

(event OnComponentBeginOverlap(OpenDoorTriggerBox)
  (params (OverlappedComponent :type Primitive%20Component%20Object%20Reference) (OtherActor :type Actor%20Object%20Reference) (OtherComp :type Primitive%20Component%20Object%20Reference) (OtherBodyIndex :type Integer) (bFromSweep :type Boolean) (SweepResult :type Hit%20Result%20Structure%20%28by%20ref%29))
  (bind _returnvalue (Game|Player|GetPlayerPawn 0))
  ;[1 1 1] Begin/End Overlap
  ;;[1 1 1] OpenDoorTriggerBox
  (if (== OtherActor _returnvalue)
    (Variables|Default|SetIsCanInteract true)
    ;;;[1 1 1] Sends To Main Character
    (Class|BPIInteracte|CanInteract(Message) _returnvalue)))

(event OnComponentBeginOverlap(DoorBoxBack)
  (params (OverlappedComponent :type Primitive%20Component%20Object%20Reference) (OtherActor :type Actor%20Object%20Reference) (OtherComp :type Primitive%20Component%20Object%20Reference) (OtherBodyIndex :type Integer) (bFromSweep :type Boolean) (SweepResult :type Hit%20Result%20Structure%20%28by%20ref%29))
  ;[1 1 1] Begin/End Overlap
  ;;[1 1 1] CheckPlayerCollisionBox
  (if (== OtherActor (Game|Player|GetPlayerPawn 0))
    (Variables|Default|SetIsPlayerInCheckBoxBack true)
    (CallFunction|CheckSetandActivateSoundifinRoomMore0EntitiesforManyRoom (Variables|Default|GetFrontBoxesCollisionForCheckEnemy))))

(event OnComponentEndOverlap(OpenDoorTriggerBox)
  (params (OverlappedComponent :type Primitive%20Component%20Object%20Reference) (OtherActor :type Actor%20Object%20Reference) (OtherComp :type Primitive%20Component%20Object%20Reference) (OtherBodyIndex :type Integer))
  (bind _returnvalue (Game|Player|GetPlayerPawn 0))
  ;[1 1 1] Begin/End Overlap
  ;;[1 1 1] OpenDoorTriggerBox
  (if (== OtherActor _returnvalue)
    (Variables|Default|SetIsCanInteract false)
    ;;;[1 1 1] Sends To Main Character
    (Class|BPIInteracte|CanNotInteract(Message) _returnvalue)))

(event OnComponentEndOverlap(DoorBoxFront)
  (params (OverlappedComponent :type Primitive%20Component%20Object%20Reference) (OtherActor :type Actor%20Object%20Reference) (OtherComp :type Primitive%20Component%20Object%20Reference) (OtherBodyIndex :type Integer))
  ;[1 1 1] Begin/End Overlap
  ;;[1 1 1] CheckPlayerCollisionBox
  (if (== OtherActor (Game|Player|GetPlayerPawn 0))
    (Variables|Default|SetIsPlayerInCheckBoxFront false)
    (CallFunction|CheckSetandActivateSoundifinRoomMore0EntitiesforManyRoom (Variables|Default|GetBackBoxesCollisionForCheckEnemy))))

(event OnComponentEndOverlap(DoorBoxBack)
  (params (OverlappedComponent :type Primitive%20Component%20Object%20Reference) (OtherActor :type Actor%20Object%20Reference) (OtherComp :type Primitive%20Component%20Object%20Reference) (OtherBodyIndex :type Integer))
  ;[1 1 1] Begin/End Overlap
  ;;[1 1 1] CheckPlayerCollisionBox
  (if (== OtherActor (Game|Player|GetPlayerPawn 0))
    (Variables|Default|SetIsPlayerInCheckBoxBack false)
    (CallFunction|CheckSetandActivateSoundifinRoomMore0EntitiesforManyRoom (Variables|Default|GetFrontBoxesCollisionForCheckEnemy))))

(event Custom|StopHearing
  (bind _isopenfront (Utilities|IsPlayerPawnPerpendiculartoDoor))
  (bind _sceneback (Variables|Default|GetSceneBack))
  (bind _scenefront (Variables|Default|GetSceneFront))
  (bind _returnvalue (select _isopenfront _scenefront _sceneback))
  (bind _returnvalue_2 (Transformation|GetWorldTransform _returnvalue))
  ;[1 1 1] EventInteract
  ;;[1 1 1] Smooth Place Player Camera Next to Door For Hearing
  (bind (_direction _newtrack_0) (Timeline|Timeline_1 Reverse)
    (:Update
      (Transformation|SetWorldLocationAndRotation (Variables|/Game/DinoAndFriends/Blueprints/MainCharacter/BP_MainCharacter.BP_MainCharacter_C|GetPlayerCamera (Variables|Default|GetAs%20Main%20Character)) (Math|Interpolation|VInterpTo (Variables|Default|GetPlayerCameraLocOnStartHearing) (.location _returnvalue_2) _newtrack_0 1.0) (Math|Interpolation|RInterpTo (Variables|Default|GetPlayerCameraRotOnStartHearing) (.rotation _returnvalue_2) _newtrack_0 1.0) false false))
    (:Finished
      (switch Utilities|FlowControl|Switch|SwitchonETimelineDirection _direction
        (:Forward
          (Variables|Default|SetIsHearingOn true)
          (Utilities|CheckRoom)
          ;;[1 1 1] Half Open Or Close Door For Hearing
          (bind (_direction_2 _halfopeninfront _halfopenback) (Timeline|Timeline_3 Play)
            (:Update
              (Transformation|SetRelativeRotation (Variables|Default|GetDoorSceneRight) (Math|Rotator|MakeRotator 0.0 0.0 (Math|Float|SelectFloat _halfopeninfront _halfopenback (Utilities|IsPlayerPawnPerpendiculartoDoor))) false false))
            (:Finished
              (switch Utilities|FlowControl|Switch|SwitchonETimelineDirection _direction_2
                (:Forward
                  ;;[1 1 1] Set Sound Based On What Jind Of Entity In Room
                  (Components|Activation|Activate (Variables|Default|GetNoiseAudio) false)
                  (if (Variables|Default|GetIsEnemyInRelativeRoom)
                    (Audio|Components|Audio|SetSound (Variables|Default|GetNoiseAudio) (Variables|Default|GetEnemyInRoomSound))
                    (elif (Variables|Default|GetIsNoiseEmmiterInRelativeRoom)
                      (Audio|Components|Audio|SetSound (Variables|Default|GetNoiseAudio) (Variables|Default|GetEnviroentSound))
                      (else
                        (Audio|Components|Audio|SetSound (Variables|Default|GetNoiseAudio) 0)))))
                (:Backward
                  (CallFunction|StopHearing))))))
        (:Backward
          (Variables|Default|SetIsHearingOn false)
          (Utilities|ReturnControl
            (:Output
              (Utilities|CheckRoom))))))))

(event Custom|PlayHearingSoundBsrdOnEntity
  ;[1 1 1] EventInteract
  ;;[1 1 1] Set Sound Based On What Jind Of Entity In Room
  (Components|Activation|Activate (Variables|Default|GetNoiseAudio) false)
  (if (Variables|Default|GetIsEnemyInRelativeRoom)
    (Audio|Components|Audio|SetSound (Variables|Default|GetNoiseAudio) (Variables|Default|GetEnemyInRoomSound))
    (elif (Variables|Default|GetIsNoiseEmmiterInRelativeRoom)
      (Audio|Components|Audio|SetSound (Variables|Default|GetNoiseAudio) (Variables|Default|GetEnviroentSound))
      (else
        (Audio|Components|Audio|SetSound (Variables|Default|GetNoiseAudio) 0)))))

(event Custom|OpenCloseDoor
  ;[1 1 1] EventInteract
  ;;[1 1 1] Just Open Door
  (if (Variables|Default|GetIsCanInteract)
    (if (Variables|Default|GetIsDoorOpen)
      (Variables|Default|SetIsDoorOpen false)
      (bind (_direction _openrightfront _openrightback) (Timeline|Timeline_0 Reverse)
        (:Update
          (bind _output_get (Variables|Default|SetDoorOpenAngle (Utilities|SelectOpenRightDoorAngle (Variables|Default|GetDoorOpenAngle) _openrightfront _openrightback)))
          (Transformation|SetRelativeRotation (Variables|Default|GetDoorSceneRight) (Math|Rotator|MakeRotator 0.0 0.0 _output_get) false false)
          (Utilities|FlowControl|DoOnce false :!label _label
            (:Completed
              (Collision|SetCollisionEnabled (Variables|Default|GetDoorMesh) "NoCollision"))))
        (:Finished
          (Collision|SetCollisionEnabled (Variables|Default|GetDoorMesh) "QueryAndPhysics")
          (goto _label Reset)))
      (else
        (Variables|Default|SetIsDoorOpen true)
        (Timeline|Timeline_0 Play)))))

(event Custom|CastToMainCharacter
  ;[1 1 1] BeginPlay
  (bind _asbp_main_character (Utilities|Casting|CastToBP_MainCharacter (Game|Player|GetPlayerPawn 0)))
  (Variables|Default|SetAs%20Main%20Character _asbp_main_character))

(event Custom|CloseHalfOpenDoor
  ;[1 1 1] EventInteract
  (if (Variables|Default|GetIsCanInteract)
    (if (not (Variables|Default|GetIsDoorOpen))
      (if (Variables|Default|GetIsHearingOn)
        ;;[1 1 1] Half Open Or Close Door For Hearing
        (bind (_direction _halfopeninfront _halfopenback) (Timeline|Timeline_3 Reverse)
          (:Update
            (Transformation|SetRelativeRotation (Variables|Default|GetDoorSceneRight) (Math|Rotator|MakeRotator 0.0 0.0 (Math|Float|SelectFloat _halfopeninfront _halfopenback (Utilities|IsPlayerPawnPerpendiculartoDoor))) false false))
          (:Finished
            (switch Utilities|FlowControl|Switch|SwitchonETimelineDirection _direction
              (:Forward
                ;;[1 1 1] Set Sound Based On What Jind Of Entity In Room
                (Components|Activation|Activate (Variables|Default|GetNoiseAudio) false)
                (if (Variables|Default|GetIsEnemyInRelativeRoom)
                  (Audio|Components|Audio|SetSound (Variables|Default|GetNoiseAudio) (Variables|Default|GetEnemyInRoomSound))
                  (elif (Variables|Default|GetIsNoiseEmmiterInRelativeRoom)
                    (Audio|Components|Audio|SetSound (Variables|Default|GetNoiseAudio) (Variables|Default|GetEnviroentSound))
                    (else
                      (Audio|Components|Audio|SetSound (Variables|Default|GetNoiseAudio) 0)))))
              (:Backward
                (CallFunction|StopHearing)))))
        (else
          (CallFunction|StopHearing))))))

(event Custom|HalfOpenDoorForHearing
  (bind _isopenfront (Utilities|IsPlayerPawnPerpendiculartoDoor))
  (bind _sceneback (Variables|Default|GetSceneBack))
  (bind _as_main_character (Variables|Default|GetAs%20Main%20Character))
  (bind _scenefront (Variables|Default|GetSceneFront))
  (bind _returnvalue (select _isopenfront _scenefront _sceneback))
  (bind _playercamera (Variables|/Game/DinoAndFriends/Blueprints/MainCharacter/BP_MainCharacter.BP_MainCharacter_C|GetPlayerCamera _as_main_character))
  (bind _returnvalue_2 (Transformation|GetWorldTransform _playercamera))
  (bind _returnvalue_3 (Transformation|GetWorldTransform _returnvalue))
  ;[1 1 1] EventInteract
  (if (Variables|Default|GetIsCanInteract)
    (if (not (Variables|Default|GetIsDoorOpen))
      ;;[1 1 1] Smooth Place Player Camera Next to Door For Hearing
      (Utilities|DisableControl)
      (Variables|Default|SetPlayerCameraLocOnStartHearing (.location _returnvalue_2))
      (Variables|Default|SetPlayerCameraRotOnStartHearing (.rotation _returnvalue_2))
      (bind (_direction _newtrack_0) (Timeline|Timeline_1 Play)
        (:Update
          (Transformation|SetWorldLocationAndRotation _playercamera (Math|Interpolation|VInterpTo (Variables|Default|GetPlayerCameraLocOnStartHearing) (.location _returnvalue_3) _newtrack_0 1.0) (Math|Interpolation|RInterpTo (Variables|Default|GetPlayerCameraRotOnStartHearing) (.rotation _returnvalue_3) _newtrack_0 1.0) false false))
        (:Finished
          (switch Utilities|FlowControl|Switch|SwitchonETimelineDirection _direction
            (:Forward
              (Variables|Default|SetIsHearingOn true)
              (Utilities|CheckRoom)
              ;;[1 1 1] Half Open Or Close Door For Hearing
              (bind (_direction_2 _halfopeninfront _halfopenback) (Timeline|Timeline_3 Play)
                (:Update
                  (Transformation|SetRelativeRotation (Variables|Default|GetDoorSceneRight) (Math|Rotator|MakeRotator 0.0 0.0 (Math|Float|SelectFloat _halfopeninfront _halfopenback (Utilities|IsPlayerPawnPerpendiculartoDoor))) false false))
                (:Finished
                  (switch Utilities|FlowControl|Switch|SwitchonETimelineDirection _direction_2
                    (:Forward
                      ;;[1 1 1] Set Sound Based On What Jind Of Entity In Room
                      (Components|Activation|Activate (Variables|Default|GetNoiseAudio) false)
                      (if (Variables|Default|GetIsEnemyInRelativeRoom)
                        (Audio|Components|Audio|SetSound (Variables|Default|GetNoiseAudio) (Variables|Default|GetEnemyInRoomSound))
                        (elif (Variables|Default|GetIsNoiseEmmiterInRelativeRoom)
                          (Audio|Components|Audio|SetSound (Variables|Default|GetNoiseAudio) (Variables|Default|GetEnviroentSound))
                          (else
                            (Audio|Components|Audio|SetSound (Variables|Default|GetNoiseAudio) 0)))))
                    (:Backward
                      (CallFunction|StopHearing))))))
            (:Backward
              (Variables|Default|SetIsHearingOn false)
              (Utilities|ReturnControl
                (:Output
                  (Utilities|CheckRoom))))))))))

(event EventBeginPlay
  ;[1 1 1] BeginPlay
  (Variables|Default|SetOutputColor (Utilities|Struct|MakeLinearColor (Math|Random|RandomFloat) (Math|Random|RandomFloat) (Math|Random|RandomFloat) 1.0))
  (CallFunction|CasttoMainCharacter))

(event EventOnTriggerBoxEndOverlapbyEntity
  (params (TriggerBox :type BP%20Room%20Trigger%20Box%20Object%20Reference) (Entity :type Actor%20Object%20Reference))
  ;[1 1 1] Begin/End Overlap
  ;;[1 1 1] CheckPlayerCollisionBox
  (CallFunction|SetWhoinRoom)
  (if (and (Utilities|Array|ContainsItem (Variables|Default|GetFrontBoxesCollisionForCheckEnemy) TriggerBox) (Variables|Default|GetIsPlayerInCheckBoxBack))
    (CallFunction|SetNoneSound :!label _label)
    (elif (and (Utilities|Array|ContainsItem (Variables|Default|GetBackBoxesCollisionForCheckEnemy) TriggerBox) (Variables|Default|GetIsPlayerInCheckBoxFront))
      (goto _label))))

(event EventSendPressedTime
  (params (PressedTime :type Float%20%28single-precision%29))
  ;[1 1 1] Interact
  (Variables|Default|SetPressed%20Time PressedTime)
  (Utilities|FlowControl|Gate true
    (:Exit
      (if (>= (Variables|Default|GetPressed%20Time) 0.5)
        (Utilities|FlowControl|DoOnce false
          (:Completed
            (CallFunction|HalfOpenDoorforHearing)))))))

(event EventOnPressedInteract
  ;[1 1 1] Interact
  (Utilities|FlowControl|Gate true) ; enters at Open
)

(event EventOnInteractButtonReleased
  ;[1 1 1] Interact
  (Utilities|FlowControl|Sequence
    (:then_0
      (Utilities|FlowControl|Gate true) ; enters at Close
    )
    (:then_1
      (Utilities|FlowControl|DoOnce false) ; enters at Reset
    )
    (:then_2
      (if (<= (Variables|Default|GetPressed%20Time) 0.2)
        (CallFunction|OpenCloseDoor)
        (else
          (CallFunction|CloseHalfOpenDoor))))))

(event EventOnTriggerBoxBeginOverlapbyEntity
  (params (TriggerBox :type BP%20Room%20Trigger%20Box%20Object%20Reference) (Entity :type Actor%20Object%20Reference))
  ;[1 1 1] Begin/End Overlap
  ;;[1 1 1] CheckPlayerCollisionBox
  (CallFunction|SetWhoinRoom Entity)
  (if (Variables|Default|GetIsHearingOn)
    (if (Variables|Default|GetIsEnemyInRelativeRoom)
      (Audio|Components|Audio|SetSound (Variables|Default|GetNoiseAudio) (Variables|Default|GetEnemyInRoomSound))
      (CallFunction|TurnonSound)
      (elif (Variables|Default|GetIsNoiseEmmiterInRelativeRoom)
        (Audio|Components|Audio|SetSound (Variables|Default|GetNoiseAudio) (Variables|Default|GetEnviroentSound))
        (CallFunction|TurnonSound)
        (else
          (CallFunction|SetNoneSound))))
    (elif (and (Utilities|Array|ContainsItem (Variables|Default|GetFrontBoxesCollisionForCheckEnemy) TriggerBox) (Variables|Default|GetIsPlayerInCheckBoxBack))
      (CallFunction|SetNailSound :!label _label)
      (CallFunction|TurnonSound)
      (elif (and (Utilities|Array|ContainsItem (Variables|Default|GetBackBoxesCollisionForCheckEnemy) TriggerBox) (Variables|Default|GetIsPlayerInCheckBoxFront))
        (goto _label)
        (else
          (CallFunction|SetNoneSound))))))

(fn ConstructionScript
  (if (Variables|Default|GetIsItADoubleDoor)
    (Components|StaticMesh|SetStaticMesh (Variables|Default|GetDoorMesh) "/Game/DinoAndFriends/StarterContent/Props/SM_Door.SM_Door")
    (Components|StaticMesh|SetStaticMesh (Variables|Default|GetDoorFrameMesh) "/Game/DinoAndFriends/StarterContent/Props/SM_DoorFrame.SM_DoorFrame")
    (else
      (Components|StaticMesh|SetStaticMesh (Variables|Default|GetDoorMesh) "/Game/DinoAndFriends/StarterContent/Props/SM_Door.SM_Door")
      (Components|StaticMesh|SetStaticMesh (Variables|Default|GetDoorFrameMesh) "/Game/DinoAndFriends/StarterContent/Props/SM_DoorFrame.SM_DoorFrame")
      (for _array_element (Variables|Default|GetFrontBoxesCollisionForCheckEnemy)
        (Utilities|Array|Add (Variables|/Game/DinoAndFriends/Blueprints/Ineractable/Door/BP_RoomTriggerBox.BP_RoomTriggerBox_C|GetRelativeDoors _array_element) self))
      (for _array_element_2 (Variables|Default|GetBackBoxesCollisionForCheckEnemy)
        (Utilities|Array|Add (Variables|/Game/DinoAndFriends/Blueprints/Ineractable/Door/BP_RoomTriggerBox.BP_RoomTriggerBox_C|GetRelativeDoors _array_element_2) self)))))

(fn TraceCheckforEntities
  (params (TriggerBox :type BP%20Room%20Trigger%20Box%20Object%20Reference))
  (bind _box (Variables|/Game/DinoAndFriends/Blueprints/Ineractable/Door/BP_RoomTriggerBox.BP_RoomTriggerBox_C|GetBox TriggerBox))
  (bind _returnvalue (Transformation|GetWorldTransform _box))
  (if (Utilities|IsValid TriggerBox)
    (bind _outhits (Class|KismetSystemLibrary|BoxTraceMulti (.location _returnvalue) (.location _returnvalue) (Components|Box|GetScaledBoxExtent _box) (Transformation|GetWorldRotation _box) "TraceTypeQuery4" false 0 "ForDuration" true "(R=1.000000,G=0.000000,B=0.000000,A=1.000000)" "(R=0.000000,G=1.000000,B=0.000000,A=1.000000)" 0.1))
    (return (> (Utilities|Array|Length _outhits) 0) _outhits)))

(fn SetWhoinRoom
  (params (InputPin :type Actor%20Object%20Reference))
  (Utilities|FlowControl|Sequence
    (:then_0
      (Utilities|IsValid InputPin
        (:Is%20Valid
          (if (Actor|ActorHasTag InputPin "Player")
            (Variables|Default|SetIsPlayerInRelativeRoom true)
            (else
              (Variables|Default|SetIsPlayerInRelativeRoom false)
              (if (Actor|ActorHasTag InputPin "Enemy")
                (Variables|Default|SetIsEnemyInRelativeRoom true)
                (else
                  (Variables|Default|SetIsEnemyInRelativeRoom false)
                  (if (Actor|ActorHasTag InputPin "NoiseEmmiter")
                    (Variables|Default|SetIsNoiseEmmiterInRelativeRoom true)
                    (else
                      (Variables|Default|SetIsNoiseEmmiterInRelativeRoom false))))))))))
    (:then_1
      (for _array_element (Variables|/Script/Engine.Actor|GetTags InputPin)
        (Development|PrintString (Utilities|String|ToString(Name) _array_element))))))

(fn SetNailSound
  (Audio|Components|Audio|SetSound (Variables|Default|GetNoiseAudio) (Variables|Default|GetNailHorrorSound)))

(fn SetNoneSound
  (Audio|Components|Audio|SetSound (Variables|Default|GetNoiseAudio) 0))

(fn TurnonSound
  (bind _noiseaudio (Variables|Default|GetNoiseAudio))
  (if (not (Components|Activation|IsActive _noiseaudio))
    (Components|Activation|Activate _noiseaudio false)))

(fn CheckSetandActivateSoundifinRoomMore0EntitiesforManyRoom
  (params (TriggerBox :type Array%20of%20BP%20Room%20Trigger%20Box%20Object%20References))
  (for _array_element TriggerBox
    (bind (_ismorethenzeroentities _outhits) (CallFunction|TraceCheckforEntities _array_element))
    (for _array_element_2 _outhits
      (CallFunction|SetWhoinRoom (.HitActor (Collision|BreakHitResult _array_element_2))))
    (if _ismorethenzeroentities
      (if (not (== (Variables|Default|GetNailHorrorSound) (Variables|/Script/Engine.AudioComponent|GetSound (Variables|Default|GetNoiseAudio))))
        (CallFunction|SetNailSound)
        (CallFunction|TurnonSound))
      (else
        (CallFunction|SetNoneSound)))))

(fn SetWhoRestinRoom
  (params (InputPin :type Actor%20Object%20Reference))
  (if (Actor|ActorHasTag InputPin "Player")
    (Variables|Default|SetIsPlayerInRelativeRoom false)
    (elif (Actor|ActorHasTag InputPin "Enemy")
      (Variables|Default|SetIsEnemyInRelativeRoom false)
      (elif (Actor|ActorHasTag InputPin "NoiseEmmiter")
        (Variables|Default|SetIsNoiseEmmiterInRelativeRoom false)))))