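; Interactable door, named as non-playable, that toggles its open state through an interact interface and records which way it opens.
; On opening, it stores the yaw of the level's BP_CheckDoorOpenWay actor and dots that facing, turned 90 degrees, against its forward vector to set front or back.
; Left and right boxes set a can-interact flag, but the live interact event ignores it.
; No door movement happens in this graph.
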(event OnComponentBeginOverlap(BoxLeft)
  (params (OverlappedComponent :type Primitive%20Component%20Object%20Reference) (OtherActor :type Actor%20Object%20Reference) (OtherComp :type Primitive%20Component%20Object%20Reference) (OtherBodyIndex :type Integer) (bFromSweep :type Boolean) (SweepResult :type Hit%20Result%20Structure%20%28by%20ref%29))
  ;[1 1 1] Begin/End Overlap
  (if (== OtherActor (Game|Player|GetPlayerPawn 0))
    (Variables|Default|SetIsCanInteract true)))

(event OnComponentBeginOverlap(BoxRight)
  (params (OverlappedComponent :type Primitive%20Component%20Object%20Reference) (OtherActor :type Actor%20Object%20Reference) (OtherComp :type Primitive%20Component%20Object%20Reference) (OtherBodyIndex :type Integer) (bFromSweep :type Boolean) (SweepResult :type Hit%20Result%20Structure%20%28by%20ref%29))
  ;[1 1 1] Begin/End Overlap
  (if (== OtherActor (Game|Player|GetPlayerPawn 0))
    (Variables|Default|SetIsCanInteract true)))

(event OnComponentEndOverlap(BoxLeft)
  (params (OverlappedComponent :type Primitive%20Component%20Object%20Reference) (OtherActor :type Actor%20Object%20Reference) (OtherComp :type Primitive%20Component%20Object%20Reference) (OtherBodyIndex :type Integer))
  ;[1 1 1] Begin/End Overlap
  (if (== OtherActor "/Game/DinoAndFriends/Blueprints/MainCharacter/BP_MainCharacter.BP_MainCharacter")
    (Variables|Default|SetIsCanInteract false)))

(event OnComponentEndOverlap(BoxRight)
  (params (OverlappedComponent :type Primitive%20Component%20Object%20Reference) (OtherActor :type Actor%20Object%20Reference) (OtherComp :type Primitive%20Component%20Object%20Reference) (OtherBodyIndex :type Integer))
  ;[1 1 1] Begin/End Overlap
  (if (== OtherActor "/Game/DinoAndFriends/Blueprints/MainCharacter/BP_MainCharacter.BP_MainCharacter")
    (Variables|Default|SetIsCanInteract false)))

(event EventInteractInterfaceFunc
  ;[1 1 1] EventInteract
  (if (Variables|Default|GetIsDoorOpen)
    (Variables|Default|SetIsDoorOpen false)
    (else
      (Variables|Default|SetIsDoorOpen true)
      (Variables|Default|SetAngleOnOpen (.Yaw (Math|Rotator|BreakRotator (.rotation (Transformation|GetActorTransform (stale EventBeginPlay _ascheck_door_open_way))))))
      (if (> (Math|Vector|DotProduct (Math|Vector|GetForwardVector (Math|Rotator|MakeRotator (.roll (Transformation|GetActorRotation (stale EventBeginPlay _ascheck_door_open_way))) (.pitch (Transformation|GetActorRotation (stale EventBeginPlay _ascheck_door_open_way))) (+ (.yaw (Transformation|GetActorRotation (stale EventBeginPlay _ascheck_door_open_way))) 9e+01))) (Transformation|GetActorForwardVector)) 0.0)
        (Variables|Default|SetIsDoorOpenFront true)
        (else
          (Variables|Default|SetIsDoorOpenFront false))))))

(event EventBeginPlay
  ;[1 1 1] EventInteract
  (Variables|Default|SetOutputColor (Utilities|Struct|MakeLinearColor (Math|Random|RandomFloat) (Math|Random|RandomFloat) (Math|Random|RandomFloat) 1.0))
  (bind _returnvalue (Actor|GetActorOfClass "/Game/DinoAndFriends/Blueprints/Ineractable/Door/BP_CheckDoorOpenWay.BP_CheckDoorOpenWay_C"))
  (bind _ascheck_door_open_way (Utilities|Casting|CastToBP_CheckDoorOpenWay _returnvalue)))

(fn ConstructionScript)