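; Interactable double door that the player toggles open and closed while inside the BoxRight trigger.
; A timeline swings both leaves, choosing front or back yaw from current angle and player side, with the right leaf's collision disabled during motion.
; An eavesdropping mode, using timelines to blend the camera and half-open the right leaf while locking player control, is present but its start logic is disconnected.
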(event OnComponentBeginOverlap(BoxRight)
  (params (OverlappedComponent :type Primitive%20Component%20Object%20Reference) (OtherActor :type Actor%20Object%20Reference) (OtherComp :type Primitive%20Component%20Object%20Reference) (OtherBodyIndex :type Integer) (bFromSweep :type Boolean) (SweepResult :type Hit%20Result%20Structure%20%28by%20ref%29))
  ;[1 1 1] Begin/End Overlap
  (if (== OtherActor (Game|Player|GetPlayerPawn 0))
    (Variables|Default|SetIsCanInteract true)))

(event OnComponentEndOverlap(BoxRight)
  (params (OverlappedComponent :type Primitive%20Component%20Object%20Reference) (OtherActor :type Actor%20Object%20Reference) (OtherComp :type Primitive%20Component%20Object%20Reference) (OtherBodyIndex :type Integer))
  ;[1 1 1] Begin/End Overlap
  (if (== OtherActor (Game|Player|GetPlayerPawn 0))
    (Variables|Default|SetIsCanInteract false)))

(event Custom|StopHearing
  (bind _isopenfront (Utilities|IsPlayerPawnPerpendiculartoDoor))
  (bind _scenefront (Variables|Default|GetSceneFront))
  (bind _sceneback (Variables|Default|GetSceneBack))
  (bind _returnvalue (select _isopenfront _scenefront _sceneback))
  (bind _returnvalue_2 (Transformation|GetWorldTransform _returnvalue))
  ;[1 1 1] EventInteract
  (bind (_direction _newtrack_0) (Timeline|Timeline_1 Reverse)
    (:Update
      (Transformation|SetWorldLocationAndRotation (Variables|/Game/DinoAndFriends/Blueprints/MainCharacter/BP_MainCharacter.BP_MainCharacter_C|GetPlayerCamera (Variables|Default|GetAs%20Main%20Character)) (Math|Interpolation|VInterpTo (Variables|Default|GetPlayerCameraLocOnStartHearing) (.location _returnvalue_2) _newtrack_0 1.0) (Math|Interpolation|RInterpTo (Variables|Default|GetPlayerCameraRotOnStartHearing) (.rotation _returnvalue_2) _newtrack_0 1.0) false false))
    (:Finished
      (if (Utilities|Enum|Equal(Enum) _direction "Forward")
        (Variables|Default|SetIsHearingOn true)
        (bind (_direction_2 _halfopeninfront _halfopenback) (Timeline|Timeline_3 Play)
          (:Update
            (Transformation|SetRelativeRotation (Variables|Default|GetDoorSceneRight) (Math|Rotator|MakeRotator 0.0 0.0 (Math|Float|SelectFloat _halfopeninfront _halfopenback (Utilities|IsPlayerPawnPerpendiculartoDoor))) false false))
          (:Finished
            (if (Utilities|Enum|Equal(Enum) _direction_2 "Backward")
              (CallFunction|StopHearing))))
        (else
          (Utilities|ReturnControl))))))

(event EventHalfOpenDoorforHearing
  ;[1 1 1] EventInteract
)

(event EventCloseHalfOpenDoor
  ;[1 1 1] EventInteract
)

(event EventInteractInterfaceFunc
  ;[1 1 1] EventInteract
  (if (Variables|Default|GetIsCanInteract)
    (if (Variables|Default|GetIsDoorOpen)
      (Variables|Default|SetIsDoorOpen false)
      (bind (_direction _openrightfront _openrightback _openleftfront _openleftback) (Timeline|Timeline_0 Reverse)
        (:Update
          (Variables|Default|SetDoorLeftOpenAngle (Utilities|SelectOpenLeftDoorAngle (Variables|Default|GetDoorLeftOpenAngle) _openleftfront _openleftback))
          (bind _output_get (Variables|Default|SetDoorRightOpenAngle (Utilities|SelectOpenRightDoorAngle (Variables|Default|GetDoorRightOpenAngle) _openrightfront _openrightback)))
          (Transformation|SetRelativeRotation (Variables|Default|GetDoorSceneRight) (Math|Rotator|MakeRotator 0.0 0.0 _output_get) false false)
          (Transformation|SetRelativeRotation (Variables|Default|GetDoorSceneLeft) (Math|Rotator|MakeRotator 0.0 0.0 (Variables|Default|GetDoorLeftOpenAngle)) false false)
          (Utilities|FlowControl|DoOnce false :!label _label
            (:Completed
              (Collision|SetCollisionEnabled (Variables|Default|GetDoorRight) "NoCollision"))))
        (:Finished
          (Collision|SetCollisionEnabled (Variables|Default|GetDoorRight) "QueryAndPhysics")
          (goto _label Reset)))
      (else
        (Variables|Default|SetIsDoorOpen true)
        (Timeline|Timeline_0 Play)))))

(event EventBeginPlay
  (Variables|Default|SetOutputColor (Utilities|Struct|MakeLinearColor (Math|Random|RandomFloat) (Math|Random|RandomFloat) (Math|Random|RandomFloat) 1.0))
  (bind _asbp_main_character (Utilities|Casting|CastToBP_MainCharacter (Game|Player|GetPlayerPawn 0)))
  (Variables|Default|SetAs%20Main%20Character _asbp_main_character))

(fn ConstructionScript)