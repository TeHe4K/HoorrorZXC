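; BP_RoomTriggerBox is a trigger volume that reports entities entering and leaving it to its related doors.
; Its Box overlap events accept only components that block custom trace channel GameTraceChannel2, using collision response as an entity filter.
; For each qualifying begin or end overlap, it loops through RelativeDoors and sends an interface message passing itself and the overlapping actor, leaving the reaction to each door.
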(event OnComponentBeginOverlap(Box)
  (params (OverlappedComponent :type Primitive%20Component%20Object%20Reference) (OtherActor :type Actor%20Object%20Reference) (OtherComp :type Primitive%20Component%20Object%20Reference) (OtherBodyIndex :type Integer) (bFromSweep :type Boolean) (SweepResult :type Hit%20Result%20Structure%20%28by%20ref%29))
  (if (Utilities|Enum|Equal(Enum) (Collision|GetCollisionResponsetoChannel OtherComp "ECC_GameTraceChannel2") "ECR_Block")
    (for _array_element (Variables|Default|GetRelativeDoors)
      (Class|BPITriggerBox|OnTriggerBoxBeginOverlapbyEntity(Message) _array_element self OtherActor))))

(event OnComponentEndOverlap(Box)
  (params (OverlappedComponent :type Primitive%20Component%20Object%20Reference) (OtherActor :type Actor%20Object%20Reference) (OtherComp :type Primitive%20Component%20Object%20Reference) (OtherBodyIndex :type Integer))
  (if (Utilities|Enum|Equal(Enum) (Collision|GetCollisionResponsetoChannel OtherComp "ECC_GameTraceChannel2") "ECR_Block")
    (for _array_element (Variables|Default|GetRelativeDoors)
      (Class|BPITriggerBox|OnTriggerBoxEndOverlapbyEntity(Message) _array_element self OtherActor))))

(event EventBeginPlay)

(event Collision|EventActorBeginOverlap
  (params (OtherActor :type Actor%20Object%20Reference)))

(event EventTick
  (params (DeltaSeconds :type Float%20%28single-precision%29)))

(fn ConstructionScript)