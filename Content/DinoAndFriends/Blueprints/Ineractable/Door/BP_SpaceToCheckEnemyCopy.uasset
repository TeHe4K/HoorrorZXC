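; Room actor that manages an ambient audio component for each of its linked BP_Doors.
; The construction script spawns audio at each door's AudioScene location and maps door to component and component to active state.
; Tick deactivates a door's audio while that door is open, hearing is on or the player-in-room flag is set, otherwise reactivates it.
; A looping timer calls an empty scan event; the player, enemy and noise-emitter detection logic is disconnected.
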(event Custom|CheckIsAnyOneInRoom
  ;[1 1 1] Scan Room For Entity
)

(event EventBeginPlay
  ;[1 1 1] Begin Play
  (Utilities|Time|SetTimerbyFunctionName 0 "CheckIsAnyOneInRoom" 0.1 true)
  (Variables|Default|SetText%20Color (Utilities|Struct|MakeLinearColor (Math|Random|RandomFloat) (Math|Random|RandomFloat) (Math|Random|RandomFloat) 1.0)))

(event EventTick
  (params (DeltaSeconds :type Float%20%28single-precision%29))
  ;[1 1 1] Event Tick
  ;[1 1 1] Check Is Audio Must Be Deactivated
  (Utilities|FlowControl|DoOnce false :!label _label
    (:Completed
      (for _array_element (Variables|Default|GetRelativeDoors)
        (if (Math|Boolean|ORBoolean (Variables|/Game/DinoAndFriends/Blueprints/Ineractable/Door/BP_Door.BP_Door_C|GetIsHearingOn _array_element) (Variables|/Game/DinoAndFriends/Blueprints/Ineractable/Door/BP_Door.BP_Door_C|GetIsDoorOpen _array_element) (Variables|Default|GetIsPlayerInThisRoom))
          ;[1 1 1] Deactivate Audio If That Activated
          (if (.Value (Utilities|Map|Find (Variables|Default|GetAudioAndActivation) (.Value (Utilities|Map|Find (Variables|Default|GetAudiosRelateToDoors) _array_element))))
            (Components|Activation|Deactivate (.Value (Utilities|Map|Find (Variables|Default|GetAudiosRelateToDoors) _array_element)))
            (Utilities|Map|Add (Variables|Default|GetAudioAndActivation) (.Value (Utilities|Map|Find (Variables|Default|GetAudiosRelateToDoors) _array_element)) false))
          (else
            ;[1 1 1] Activate Audio If That Not Activated Yet
            (if (not (.Value (Utilities|Map|Find (Variables|Default|GetAudioAndActivation) (.Value (Utilities|Map|Find (Variables|Default|GetAudiosRelateToDoors) _array_element)))))
              (Components|Activation|Activate (.Value (Utilities|Map|Find (Variables|Default|GetAudiosRelateToDoors) _array_element)) false)
              (Utilities|Map|Add (Variables|Default|GetAudioAndActivation) (.Value (Utilities|Map|Find (Variables|Default|GetAudiosRelateToDoors) _array_element)) true)))))
      (goto _label Reset))))

(fn ConstructionScript
  (for _array_element (Variables|Default|GetRelativeDoors)
    (bind _asbp_door (Utilities|Casting|CastToBP_Door _array_element))
    (bind _returnvalue (AddComponent|AddAudioComponent true (Math|Transform|MakeTransform (Transformation|GetWorldLocation (Variables|/Game/DinoAndFriends/Blueprints/Ineractable/Door/BP_Door.BP_Door_C|GetAudioScene _asbp_door)) "0, 0, 0" "1,1,1")))
    (Utilities|Map|Add (Variables|Default|GetAudiosRelateToDoors) _asbp_door _returnvalue)
    (Utilities|Map|Add (Variables|Default|GetAudioAndActivation) _returnvalue true)))