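; BP_MainCharacter1 is a first-person-style player character with walk, look, jump, crouch, run and a toggleable flashlight with sounds.
; Run offsets max walk speed by an acceleration value, movement axes are gated by IsCanMove, and forward input also feeds TurnRateForDoorFromOutlast.
; CanInteract and CanNotInteract toggle the interactable widget's visibility.
; Interaction is unfinished: a short camera trace stores the hit actor, while tap-versus-hold "hearing" logic is disconnected.
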(event Custom|InteractEvent
  (params (IsHearing :type Boolean))
  (bind _playercamera (Variables|Pawn|GetPlayerCamera))
  (bind _returnvalue (Transformation|GetWorldLocation _playercamera))
  ;[1 1 1] Interact
  (bind (_outhit _returnvalue_2) (Collision|LineTraceByChannel _returnvalue (+ _returnvalue (* (Math|Vector|GetForwardVector _playercamera) 125.0)) "TraceTypeQuery3" false 0 "None"))
  (if _returnvalue_2
    (Variables|Default|SetInteractActor (.HitActor (Collision|BreakHitResult _outhit)))
    (if IsHearing
      _)))

(event EventCanInteract
  ;[1 1 1] TriggedWDVisibility
  (bind _foundwidgets (Widget|GetAllWidgetsOfClass "/Game/DinoAndFriends/UI/MainCharacterHUD/WDBP_Interactable.WDBP_Interactable_C" false))
  (Widget|SetVisibility (Utilities|Array|Get(acopy) _foundwidgets) "HitTestInvisible"))

(event EventCanNotInteract
  ;[1 1 1] TriggedWDVisibility
  (bind _foundwidgets (Widget|GetAllWidgetsOfClass "/Game/DinoAndFriends/UI/MainCharacterHUD/WDBP_Interactable.WDBP_Interactable_C" false))
  (Widget|SetVisibility (Utilities|Array|Get(acopy) _foundwidgets) "Collapsed"))

(event EventBeginPlay)

(event Input|ActionEvents|InputActionJump
  (params (Key :type Key%20Structure :default "None"))
  ;[1 1 1] MovementActions
  (:Pressed
    (Character|Jump)))

(event Input|ActionEvents|InputActionCrounch
  (params (Key :type Key%20Structure :default "None"))
  ;[1 1 1] MovementActions
  (:Pressed
    (Character|Crouch))
  (:Released
    (Character|UnCrouch)))

(event Input|ActionEvents|InputActionRun
  (params (Key :type Key%20Structure :default "None"))
  (bind _charactermovement (Variables|Character|GetCharacterMovement))
  (bind _charactermovement_2 (Variables|Character|GetCharacterMovement))
  (bind _accelerations (Variables|Default|GetAccelerations))
  ;[1 1 1] MovementActions
  (:Pressed
    (Variables|/Script/Engine.CharacterMovementComponent|SetMaxWalkSpeed _charactermovement (+ _accelerations (Class|MovementComponent|GetMaxSpeed _charactermovement_2))))
  (:Released
    (Variables|/Script/Engine.CharacterMovementComponent|SetMaxWalkSpeed _charactermovement (- (Class|MovementComponent|GetMaxSpeed _charactermovement_2) _accelerations))))

(event Input|ActionEvents|InputActionFlashlight
  (params (Key :type Key%20Structure :default "None"))
  ;[1 1 1] Flashlight
  (:Pressed
    (if (Variables|Default|GetIsFlashlightON)
      (Audio|PlaySoundatLocation "/Game/DinoAndFriends/Sounds/Flashlight/FlashLight_OFF.FlashLight_OFF" (Transformation|GetWorldLocation (Variables|Default|GetFlashLight)) "0, 0, 0" 1.0 1.0 0.0 0 0 0)
      (Rendering|SetVisibility (Variables|Default|GetFlashLight) false false)
      (Variables|Default|SetIsFlashlightON false)
      (else
        (Audio|PlaySoundatLocation "/Game/DinoAndFriends/Sounds/Flashlight/FlashLight_ON.FlashLight_ON" (Transformation|GetWorldLocation (Variables|Default|GetFlashLight)) "0, 0, 0" 1.0 1.0 0.0 0 0 0)
        (Rendering|SetVisibility (Variables|Default|GetFlashLight) true false)
        (Variables|Default|SetIsFlashlightON true)))))

(event Input|ActionEvents|InputActionInteract
  (params (Key :type Key%20Structure :default "None"))
  ;[1 1 1] Interact
  (:Released
    (Utilities|IsValid (Variables|Default|GetInteractActor))))

(event Input|AxisEvents|InputAxisMoveForwardandBack
  (params (AxisValue :type Float%20%28single-precision%29))
  ;[1 1 1] Movement
  (if (Variables|Default|GetIsCanMove)
    (Pawn|Input|AddMovementInput (Transformation|GetActorForwardVector) AxisValue false)
    (Variables|Default|SetTurnRate%28ForDoorFromOutlast%29 AxisValue)))

(event Input|AxisEvents|InputAxisMoveRightandLeft
  (params (AxisValue :type Float%20%28single-precision%29))
  ;[1 1 1] Movement
  (if (Variables|Default|GetIsCanMove)
    (Pawn|Input|AddMovementInput (Transformation|GetActorRightVector) AxisValue false)))

(event Input|AxisEvents|InputAxisLookUpandDown
  (params (AxisValue :type Float%20%28single-precision%29))
  ;[1 1 1] Camera
  (Pawn|Input|AddControllerPitchInput AxisValue))

(event Input|AxisEvents|InputAxisLookHorizontal
  (params (AxisValue :type Float%20%28single-precision%29))
  ;[1 1 1] Camera
  (Pawn|Input|AddControllerYawInput AxisValue))

(event Input|AxisEvents|InputAxisInteractLongAKAHearing
  (params (AxisValue :type Float%20%28single-precision%29))
  ;[1 1 1] Interact
  (Variables|Default|SetInteractPressedSeconds (Class|PlayerController|GetInputKeyTimeDown (Game|GetPlayerController 0) (stale Input|ActionEvents|InputActionInteract Key))))

(fn ConstructionScript)