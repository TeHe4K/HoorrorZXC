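; Interactable door, derived from a base interaction class, that opens fully on a tap or cracks ajar for peeking on a two-second hold.
; Player facing at key press picks the swing direction and which of two cameras to use.
; Timelines drive both rotations; peeking blends the view to the door and blocks character input until release.
; Peeking also box-traces nearby objects for SetSound, which is an empty stub.
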(event Custom|PressedDoor
  ;[1 1 1] Функция при зажатии
  (Utilities|FlowControl|FlipFlop
    (:A
      (Variables|Default|SetIsPressed? true)
      (bind _alpha (Timeline|Timeline_1 PlayFromStart)
        (:Update
          (Transformation|SetRelativeRotation (Variables|Default|GetDoor) (Math|Rotator|Lerp(Rotator) "0, 0, 0" (select (Variables|Default|GetForwardOpen) "0.000000,-25.000000,0.000000" "0,25.000000, 0") _alpha) false false))))
    (:B
      (Variables|Default|SetIsPressed? false)
      (Timeline|Timeline_1 Reverse))))

(event Custom|Click
  ;[1 1 1] Взаимодействие при нажатии
  (if (Variables|Default|GetIsUse)
    (CallFunction|OpenDoor)))

(event Custom|OpenDoor
  ;[1 1 1] Функция при нажатии
  (Utilities|FlowControl|FlipFlop
    (:A
      (bind _alpha (Timeline|Timeline_0 Play)
        (:Update
          (Transformation|SetRelativeRotation (Variables|Default|GetDoor) (Math|Rotator|Lerp(Rotator) "0, 0, 0" (Utilities|LerpRotate) _alpha) false false))
        (:Finished
          (Variables|Default|SetDoorRotate (Math|Rotator|Lerp(Rotator) "0, 0, 0" (Utilities|LerpRotate) _alpha))
          (if (Variables|Default|GetIsOpen)
            (Variables|Default|SetIsOpen false)
            (else
              (Variables|Default|SetIsOpen true))))))
    (:B
      (Timeline|Timeline_0 Reverse))))

(event Custom|PressedEnd
  ;[1 1 1] Конец взаимодействия зажатия
  (if (Variables|Default|GetIsUse)
    (if (not (Variables|Default|GetIsOpen))
      (Game|Player|SetViewTargetwithBlend (Game|GetPlayerController 0) (Variables|Default|GetCharacter) 1.5 "VTBlend_Linear" 0.0 true)
      (CallFunction|PressedDoor)
      (Utilities|FlowControl|Delay 1.5)
      (Variables|/Game/DinoAndFriends/Blueprints/MainCharacter/BP_MainCharacter.BP_MainCharacter_C|SetIsInputBlock (Variables|Default|GetCharacter) false)
      (Variables|Default|SetIsPressed? false)
      (CallFunction|MultyTrace))))

(event Custom|Press
  ;[1 1 1] Взаимодействие при зажатии
  (if (Variables|Default|GetIsUse)
    (if (Variables|Default|GetIsOpen)
      (CallFunction|OpenDoor)
      (else
        (CallFunction|SetCamera)
        (Game|Player|SetViewTargetwithBlend (Game|GetPlayerController 0) self 1.5 "VTBlend_Linear" 0.0 true)
        (Variables|/Game/DinoAndFriends/Blueprints/MainCharacter/BP_MainCharacter.BP_MainCharacter_C|SetIsInputBlock (Variables|Default|GetCharacter) true)
        (Variables|Default|SetIsPressed? true)
        (CallFunction|PressedDoor)
        (CallFunction|MultyTrace)))))

(event EventInteract
  (params (Character :type BP%20Main%20Character%20Object%20Reference) (Inventory :type BPC%20Inventory%20Object%20Reference))
  ;[1 1 1] Наследование от базового класса
  (|CallParentFunction Character Inventory))

(event EventEndInteract
  ;[1 1 1] Наследование от базового класса
  (|CallParentFunction))

(event Input|ActionEvents|InputActionInteract
  (params (Key :type Key%20Structure :default "None"))
  ;[1 1 1] Инпуты взаимодействия
  (:Pressed
    (Variables|Default|SetForwardOpen (Utilities|PlayerForward))
    (Utilities|FlowControl|Gate true) ; enters at Open
  )
  (:Released
    (Utilities|FlowControl|Sequence
      (:then_0
        (Utilities|FlowControl|Gate true) ; enters at Close
      )
      (:then_1
        (if (Variables|Default|GetIsPressed?)
          (CallFunction|PressedEnd)
          (else
            (CallFunction|Click)))))))

(event Input|AxisEvents|InputAxisInteract
  (params (AxisValue :type Float%20%28single-precision%29))
  ;[1 1 1] Инпуты взаимодействия
  (if (> AxisValue 0.0)
    (Utilities|FlowControl|Gate true :!label _label
      (:Exit
        (bind _output_get (Variables|Default|SetTime%20Key%20Pressed (Class|PlayerController|GetInputKeyTimeDown (Game|GetPlayerController 0) (stale Input|ActionEvents|InputActionInteract Key))))
        (if (>= _output_get 2.0)
          (if (not (Variables|Default|GetIsOpen))
            (CallFunction|Press)
            (goto _label Toggle)))))))

(fn ConstructionScript
  (|CallParentFunction))

(fn SetCamera
  (if (Variables|Default|GetForwardOpen)
    (Components|Activation|SetActive (Variables|Default|GetCamera) true false)
    (Components|Activation|SetActive (Variables|Default|GetCamera1) false false)
    (else
      (Components|Activation|SetActive (Variables|Default|GetCamera) false false)
      (Components|Activation|SetActive (Variables|Default|GetCamera1) true false))))

(fn MultyTrace
  (bind _arrow (Variables|Default|GetArrow))
  (bind _returnvalue (Transformation|GetWorldLocation _arrow))
  (bind _outhits (Class|KismetSystemLibrary|BoxTraceMultiforObjects _returnvalue (+ _returnvalue (* (Math|Vector|GetForwardVector (Variables|Default|GetArrow)) 1e+02)) "1000.000000,1000.000000,1000.000000" "0, 0, 0" (Utilities|Array|MakeArray "ObjectTypeQuery1" "ObjectTypeQuery3" "ObjectTypeQuery2" "ObjectTypeQuery4") false (Utilities|Array|MakeArray 0 self) "None" true))
  (if (== (Utilities|Array|Length _outhits) 0)
    (CallFunction|SetSound)
    (else
      (bind _array_element (Utilities|Array|ForEachLoopwithBreak _outhits)
        (:LoopBody
          (if (Utilities|DoesObjectImplementInterface (.HitActor (Collision|BreakHitResult _array_element)) 0)
            _))
        (:Completed
          (CallFunction|SetSound (Variables|Default|GetSoundObj)))))))

(fn SetSound
  (params (NewSound :type Sound%20Base%20Object%20Reference)))