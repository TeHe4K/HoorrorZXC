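; BP_ControlPanel is an interactable keypad panel that sets itself Active when the entered code matches its Password.
; While it is inactive, the interact key maps the hit component to a button by object name.
; Digit presses append to CurrentCode, restarting on overflow, and update the text display, while Accept checks the code and Reset clears it.
; Button clicks show feedback through material changes separated by a short delay.
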(event Custom|ButtonsEvent
  (params (TouchedComponent :type Primitive%20Component%20Object%20Reference))
  (bind _returnvalue (Utilities|GetObjectName TouchedComponent))
  (Variables|Default|SetTouched%20Component TouchedComponent)
  (if (Utilities|Enum|Equal(Enum) _returnvalue "Accept")
    (CallFunction|AcceptPassword)
    (elif (Utilities|Enum|Equal(Enum) _returnvalue "Reset")
      (CallFunction|ResetPassword)
      (else
        (Variables|Default|SetCurrent%20Code (Utilities|String|Append (Variables|Default|GetCurrent%20Code) (Utilities|String|ToString(Integer) (Math|Conversions|ToInteger(Byte) _returnvalue))))
        (if (> (Utilities|String|Len (Variables|Default|GetCurrent%20Code)) (Utilities|String|Len (Variables|Default|GetPassword)))
          (Variables|Default|SetCurrent%20Code "")
          (Variables|Default|SetCurrent%20Code (Utilities|String|Append (Variables|Default|GetCurrent%20Code) (Utilities|String|ToString(Integer) (Math|Conversions|ToInteger(Byte) _returnvalue)))))
        (CallFunction|SetText)
        (CallFunction|ClickButton (Variables|Default|GetTouched%20Component))
        (Utilities|FlowControl|Delay 0.2)
        (CallFunction|ClickButton (Variables|Default|GetTouched%20Component))))))

(event Custom|AcceptPassword
  (CallFunction|CheckPassword)
  (Variables|Default|SetCurrent%20Code "")
  (CallFunction|SetText))

(event Custom|ResetPassword
  (Variables|Default|SetCurrent%20Code "")
  (CallFunction|SetText)
  (CallFunction|ClickButton (Variables|Default|GetTouched%20Component))
  (Utilities|FlowControl|Delay 0.2)
  (CallFunction|ClickButton (Variables|Default|GetTouched%20Component)))

(event Custom|CheckPassword
  (if (Utilities|Enum|Equal(Enum) (Variables|Default|GetPassword) (Variables|Default|GetCurrent%20Code))
    (Variables|Default|SetActive true)
    (Variables|Default|SetCurrent%20Code "")
    (else
      (Variables|Default|SetCurrent%20Code ""))))

(event EventBeginPlay)

(event Collision|EventActorBeginOverlap
  (params (OtherActor :type Actor%20Object%20Reference)))

(event EventTick
  (params (DeltaSeconds :type Float%20%28single-precision%29)))

(event EventInteract
  (params (Character :type BP%20Main%20Character%20Object%20Reference) (Inventory :type BPC%20Inventory%20Object%20Reference))
  (|CallParentFunction Character Inventory))

(event EventEndInteract
  (|CallParentFunction))

(event Input|ActionEvents|InputActionInteractq
  (params (Key :type Key%20Structure))
  (bind _character (Variables|Default|GetCharacter))
  (bind _hitresultinteract (Variables|/Game/DinoAndFriends/Blueprints/MainCharacter/BP_MainCharacter.BP_MainCharacter_C|GetHitResultInteract _character))
  (bind _hitcomponent (Collision|BreakHitResult _hitresultinteract))
  (:Pressed
    (if (not (Variables|Default|GetActive))
      (if (!= (Variables|Default|GetControlPanel) _hitcomponent)
        (Utilities|FlowControl|Sequence
          (:then_0
            (CallFunction|ClickButton _hitcomponent)
            (Utilities|FlowControl|Delay 0.2)
            (CallFunction|ClickButton _hitcomponent))
          (:then_1
            (for _array_element (Variables|Default|GetButtons)
              (if (Utilities|Enum|Equal(Enum) (Utilities|GetObjectName _array_element) (Utilities|GetObjectName _hitcomponent))
                (CallFunction|ButtonsEvent _array_element)))))))))

(fn ConstructionScript
  (Variables|Default|SetButtons (Utilities|Array|MakeArray (Variables|Default|Get0) (Variables|Default|Get1) (Variables|Default|Get2) (Variables|Default|Get3) (Variables|Default|Get4) (Variables|Default|Get5) (Variables|Default|Get6) (Variables|Default|Get7) (Variables|Default|Get8) (Variables|Default|Get9) (Variables|Default|GetAccept) (Variables|Default|GetReset))))

(fn SetText
  (Rendering|Components|TextRender|SetText (Variables|Default|GetCode%20Text) (Utilities|Text|ToText(String) (Variables|Default|GetCurrent%20Code))))

(fn ClickButton
  (params (Target :type Primitive%20Component%20Object%20Reference) (Material :type Material%20Interface%20Object%20Reference))
  (Rendering|Material|SetMaterial Target 0 Material))