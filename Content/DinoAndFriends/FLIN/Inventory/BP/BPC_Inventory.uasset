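; BPC_Inventory is an inventory component that stores a character's items as slots of class, amount and item info.
; Adding searches for the first slot of the same class, stacking amounts if allowed or appending a new slot.
; Removal overwrites a slot's amount and deletes it at zero.
; It also opens and closes the WD_InventoryHUD widget, toggling the mouse cursor and destroying the widget slots' actors on close.
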(event EventBeginPlay)

(event EventTick
  (params (DeltaSeconds :type Float%20%28single-precision%29)))

(fn FInit
  (params (Character :type BP%20Main%20Character%20Object%20Reference))
  (Variables|Default|SetCharacter Character))

(fn FAddItem
  (params (ItemClass :type BP%20Base%20Inventory%20Actor%20Class%20Reference) (ItemInfo :type Struct%20Item%20Structure))
  (bind _amount (Utilities|Struct|BreakStruct_Item ItemInfo))
  (bind (_have _index _amount_2) (CallFunction|FSearchHaveItem ItemClass))
  (if _have
    (if (Utilities|Struct|BreakStruct_Item ItemInfo)
      (Utilities|Array|SetArrayElem (Variables|Default|GetSlots) _index (Utilities|Struct|MakeStruct_InventorySlots ItemClass (+ _amount_2 _amount) ItemInfo))
      (else
        (Utilities|Array|Add (Variables|Default|GetSlots) (Utilities|Struct|MakeStruct_InventorySlots ItemClass _amount ItemInfo) :!label _label)))
    (else
      (goto _label))))

(fn FSearchHaveItem
  (params (ItemClass :type BP%20Base%20Inventory%20Actor%20Class%20Reference))
  (bind (_array_element _array_index) (Utilities|Array|ForEachLoopwithBreak (Variables|Default|GetSlots) :!label _label)
    (:LoopBody
      (if (== (.itemclass _array_element) ItemClass)
        (LocalVariables|SetHaveL true)
        (LocalVariables|SetIndexL _array_index)
        (LocalVariables|SetAmountL (.amount _array_element))
        (goto _label Break)))
    (:Completed
      (return (LocalVariables|GetHaveL) (LocalVariables|GetIndexL) (LocalVariables|GetAmountL)))))

(fn FRemoveItem
  (params (ItemClass :type BP%20Base%20Inventory%20Actor%20Class%20Reference) (Index :type Integer) (Amount :type Integer))
  (Utilities|Array|SetArrayElem (Variables|Default|GetSlots) Index (Utilities|Struct|MakeStruct_InventorySlots ItemClass Amount (.iteminfo (Utilities|Array|Get(acopy) (Variables|Default|GetSlots) Index))))
  (if (== (.amount (Utilities|Array|Get(acopy) (Variables|Default|GetSlots) Index)) 0)
    (Utilities|Array|RemoveIndex (Variables|Default|GetSlots) Index)))

(fn FCreatInventory
  (bind _returnvalue (UserInterface|CreateWidget "/Game/DinoAndFriends/FLIN/Inventory/Widgets/WD_InventoryHUD.WD_InventoryHUD_C" 0 self))
  (bind _output_get (Variables|Default|SetWD_Inventory _returnvalue))
  (UserInterface|Viewport|AddtoViewport _output_get 0)
  (Variables|/Script/Engine.PlayerController|SetbShowMouseCursor (Game|GetPlayerController 0) true))

(fn FRemoveInventory
  (Widget|RemovefromParent (Variables|Default|GetWD_Inventory))
  (Variables|/Script/Engine.PlayerController|SetbShowMouseCursor (Game|GetPlayerController 0) false)
  (for _array_element (Variables|/Game/DinoAndFriends/FLIN/Inventory/Widgets/WD_InventoryHUD.WD_InventoryHUD_C|GetSlots (Variables|Default|GetWD_Inventory))
    (if (Utilities|IsValid (Variables|/Game/DinoAndFriends/FLIN/Inventory/Widgets/WD_SlotItem.WD_SlotItem_C|GetActor _array_element))
      (Actor|DestroyActor (Variables|/Game/DinoAndFriends/FLIN/Inventory/Widgets/WD_SlotItem.WD_SlotItem_C|GetActor _array_element)))))