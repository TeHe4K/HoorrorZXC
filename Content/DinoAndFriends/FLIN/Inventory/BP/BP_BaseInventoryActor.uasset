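; Base actor for world items that a character can pick up into an inventory.
; The construction script fills ItemInfo from the DT_Item data table row named by RowName.
; Interact stores the character and inventory and enables player input on the actor, while EndInteract disables it.
; The Interact input action then passes its class and ItemInfo to the inventory's FAddItem and destroys the actor.
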(event EventBeginPlay)

(event Collision|EventActorBeginOverlap
  (params (OtherActor :type Actor%20Object%20Reference)))

(event EventTick
  (params (DeltaSeconds :type Float%20%28single-precision%29)))

(event EventInteract
  (params (Character :type BP%20Main%20Character%20Object%20Reference) (Inventory :type BPC%20Inventory%20Object%20Reference))
  (Variables|Default|SetCharacter Character)
  (Variables|Default|SetInventory Inventory)
  (Input|EnableInput (Game|GetPlayerController 0)))

(event EventEndInteract
  (Input|DisableInput (Game|GetPlayerController 0)))

(event Input|ActionEvents|InputActionInteract
  (params (Key :type Key%20Structure :default "None"))
  (:Pressed
    (Default|FAddItem (Variables|Default|GetInventory) (Utilities|GetClass self) (Variables|Default|GetItemInfo))
    (Actor|DestroyActor)))

(fn ConstructionScript
  (bind _returnvalue (Utilities|GetDataTableRow "/Game/DinoAndFriends/FLIN/Inventory/Struck/DT_Item.DT_Item" (Variables|Default|GetRow%20Name))
    (:then
      (Variables|Default|SetItemInfo _returnvalue))))