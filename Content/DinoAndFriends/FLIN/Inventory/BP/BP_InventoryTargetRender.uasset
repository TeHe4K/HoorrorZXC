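; Inventory preview actor that films its own item meshes with a scene capture component for inspecting items.
; The capture shows only this actor's components, and VisibleItem hides every mesh before revealing the indexed one, currently just Battery.
; Holding Zoom plays a timeline that narrows the capture FOV and lets look input rotate the meshes.
; Releasing Zoom reverses the timeline and stops rotation.
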(event Custom|VisibleItem
  (params (Index :type E_ItemTarget%20Enum :default "NewEnumerator1"))
  (for _array_element (Variables|Default|GetMesh)
    (Rendering|SetVisibility _array_element false false))
  (Rendering|SetVisibility (Utilities|Select :Index Index :NewEnumerator1 (Variables|Default|GetBattery)) true false))

(event EventBeginPlay
  (Rendering|SceneCapture|ShowOnlyActorComponents (Variables|Default|GetSceneCaptureComponent2D) self false)
  (Input|EnableInput (Game|GetPlayerController 0)))

(event Collision|EventActorBeginOverlap
  (params (OtherActor :type Actor%20Object%20Reference)))

(event EventTick
  (params (DeltaSeconds :type Float%20%28single-precision%29)))

(event Input|ActionEvents|InputActionZoom
  (params (Key :type Key%20Structure :default "None"))
  (:Pressed
    (Variables|Default|SetInspect true)
    (bind _alpha (Timeline|Timeline_0 Play)
      (:Update
        (Variables|/Script/Engine.SceneCaptureComponent2D|SetFOVAngle (Variables|Default|GetSceneCaptureComponent2D) (Math|Float|Lerp 9e+01 6e+01 _alpha)))))
  (:Released
    (Variables|Default|SetInspect false)
    (Timeline|Timeline_0 Reverse)))

(event Input|AxisEvents|InputAxisLookUpandDown
  (params (AxisValue :type Float%20%28single-precision%29))
  (if (Variables|Default|GetInspect)
    (Transformation|AddLocalRotation (Variables|Default|GetMesh) (Math|Rotator|MakeRotator 0.0 0.0 (* AxisValue 1e+01)) false false)))

(event Input|AxisEvents|InputAxisLookHorizontal
  (params (AxisValue :type Float%20%28single-precision%29))
  (if (Variables|Default|GetInspect)
    (Transformation|AddLocalRotation (Variables|Default|GetMesh) (Math|Rotator|MakeRotator 0.0 (* AxisValue 1e+01) 0.0) false false)))

(fn ConstructionScript
  (Variables|Default|SetMesh (Utilities|Array|MakeArray (Variables|Default|GetBattery))))